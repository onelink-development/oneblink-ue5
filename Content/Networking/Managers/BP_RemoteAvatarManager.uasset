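; BP_RemoteAvatarManager spawns a BP_RemoteAvatar for VR players other than the local one.
; On BeginPlay it walks the GameState PlayerArray once, filtering out the local player by comparing controller player states.
; Each avatar spawns at the manager's transform with its TargetPlayerState set.
; Spawning precedes the TrackedPlayerStates check, which adds a state only if already present, so that list never gains new players here.
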(event `self.ReceiveBeginPlay`
  (bind _returnvalue (`GameplayStatics.GetPlayerController` 0))
  (for _array_element (`GameStateBase.PlayerArray` (`GameplayStatics.GetGameState`))
    (bind _asbp_vrplayer_state (cast `/Game/Networking/PlayerState/BP_VRPlayerState` _array_element))
    (if (`KismetSystemLibrary.IsValid` _returnvalue)
      (if (!= (`Controller.PlayerState` (`PlayerState.GetPlayerController` _asbp_vrplayer_state)) (`Controller.PlayerState` _returnvalue))
        (`|SpawnActorFromClass` "/Game/Networking/ReplicatedActors/BP_RemoteAvatar.BP_RemoteAvatar_C" (`self.GetTransform`) "Undefined" "MultiplyWithRoot" null _asbp_vrplayer_state null)
        (if (`KismetArrayLibrary.Array_Contains` (`self.TrackedPlayerStates`) _asbp_vrplayer_state)
          (`KismetArrayLibrary.Array_Add` (`self.TrackedPlayerStates`) _asbp_vrplayer_state))))))

(fn `UserConstructionScript`)