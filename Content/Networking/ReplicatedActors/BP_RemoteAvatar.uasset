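; BP_RemoteAvatar is an actor that visually represents another player's head and both hands, likely for a networked VR session.
; On BeginPlay it binds to head, left hand and right hand update events on its TargetPlayerState, if that reference is valid.
; Each handler copies the matching replicated transform from the player state onto its parent component in world space, without sweep, teleport or interpolation.
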(event `self.ReceiveBeginPlay`
  (`/Engine/EditorBlueprintResources/StandardMacros.IsValid` (`self.TargetPlayerState`)
    (:`Is Valid`
      (add `/Game/Networking/PlayerState/BP_VRPlayerState.OnHeadTransformUpdated` (`self.TargetPlayerState`) (delegate `UpdateHeadTransform`))
      (add `/Game/Networking/PlayerState/BP_VRPlayerState.OnLeftHandTransformUpdated` (`self.TargetPlayerState`) (delegate `UpdateLeftHandTransform`))
      (add `/Game/Networking/PlayerState/BP_VRPlayerState.OnRightHandTransformUpdated` (`self.TargetPlayerState`) (delegate `UpdateRightHandTransform`)))))

(event `UpdateRightHandTransform`
  (`SceneComponent.K2_SetWorldTransform` (`self.RightHandParent`) (`/Game/Networking/PlayerState/BP_VRPlayerState.RepRightHandTransform` (`self.TargetPlayerState`)) false false))

(event `UpdateHeadTransform`
  (`SceneComponent.K2_SetWorldTransform` (`self.HeadParent`) (`/Game/Networking/PlayerState/BP_VRPlayerState.RepHeadTransform` (`self.TargetPlayerState`)) false false))

(event `UpdateLeftHandTransform`
  (`SceneComponent.K2_SetWorldTransform` (`self.LeftHandParent`) (`/Game/Networking/PlayerState/BP_VRPlayerState.RepLeftHandTransform` (`self.TargetPlayerState`)) false false))

(fn `UserConstructionScript`)